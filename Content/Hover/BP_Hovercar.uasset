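; BP_Hovercar is a drivable hovercar steered by movement and turning input axes.
; Movement pushes the static mesh with force along the forward vector, while turning yaws the actor directly.
; Tick restarts two timelines every frame, lerping the mesh's relative roll and yaw toward turn-scaled angles for banking.
; The construction script initializes HoverComponent with the mesh and adds four corner hover points.
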(event `InputAxis|movement`
  (params (AxisValue :type "Float (single-precision)"))
  (`PrimitiveComponent.AddForce` (`self.StaticMesh`) (* (* (`SceneComponent.GetForwardVector`) 500000.0) AxisValue) "None" false))

(event `InputAxis|turning`
  (params (AxisValue :type "Float (single-precision)"))
  (`self.K2_AddActorLocalRotation` (`KismetMathLibrary.MakeRotator` 0.0 0.0 (* AxisValue 2.0))))

(event `self.ReceiveTick`
  (params (DeltaSeconds :type "Float (single-precision)"))
  (bind _returnvalue (`self.GetInputAxisValue`))
  (bind _staticmesh (`self.StaticMesh`))
  (bind _staticmesh_2 (`self.StaticMesh`))
  (bind (_relativerotation_roll _relativerotation_pitch _relativerotation_yaw) (`KismetMathLibrary.BreakRotator` (`SceneComponent.RelativeRotation` _staticmesh)))
  (bind (_relativerotation_roll_2 _relativerotation_pitch_2 _relativerotation_yaw_2) (`KismetMathLibrary.BreakRotator` (`SceneComponent.RelativeRotation` _staticmesh_2)))
  (`|ExecutionSequence`
    (:`then_0`
      (bind (_direction _newtrack_0) (`Timeline|Timeline_0` :!via `PlayFromStart`)
        (:`Update`
          (`SceneComponent.K2_SetRelativeRotation` _staticmesh_2 (`KismetMathLibrary.MakeRotator` (`KismetMathLibrary.Lerp` _relativerotation_roll_2 (`KismetMathLibrary.MapRangeUnclamped` _returnvalue -1.0 1.0 -20.0 20.0) _newtrack_0) _relativerotation_pitch_2 _relativerotation_yaw_2) false false))))
    (:`then_1`
      (bind (_direction_2 _newtrack_1) (`Timeline|Timeline_1` :!via `PlayFromStart`)
        (:`Update`
          (`SceneComponent.K2_SetRelativeRotation` _staticmesh (`KismetMathLibrary.MakeRotator` _relativerotation_roll _relativerotation_pitch (`KismetMathLibrary.Lerp` _relativerotation_yaw (`KismetMathLibrary.MapRangeUnclamped` _returnvalue -1.0 1.0 -10.0 10.0) _newtrack_1)) false false))))))

(fn `UserConstructionScript`
  (bind _hovercomponent (`self.HoverComponent`))
  (bind _pointarray (`/Game/Hover/HoverComponent.PointArray` _hovercomponent))
  (`/Game/Hover/HoverComponent.InitComponent` _hovercomponent (`self.StaticMesh`))
  (`|ExecutionSequence`
    (:`then_1`
      (`KismetArrayLibrary.Array_Add` _pointarray (160.0 70.0 0.0)))
    (:`then_2`
      (`KismetArrayLibrary.Array_Add` _pointarray (160.0 -70.0 0.0)))
    (:`then_3`
      (`KismetArrayLibrary.Array_Add` _pointarray (-160.0 70.0 0.0)))
    (:`then_4`
      (`KismetArrayLibrary.Array_Add` _pointarray (-160.0 -70.0 0.0)))))