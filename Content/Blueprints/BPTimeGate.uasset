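; Timed checkpoint gate for the player car that ends the round if its countdown expires before the car arrives.
; Car overlap updates the TimeLeftOnGate stat using the full GateTime, plays a sound, broadcasts gate reached through BI_GameEvents, then destroys the gate.
; Before destruction, it activates the other gate and starts that countdown, assuming only two gates exist at once.
; Overlap does not check IsActive, and game-over handling is marked unfinished.
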(event `setAverageTimeLeft`
  ;[1 1 1] set average time left on gate stat on player car
  (bind (_playerstats_collisions _playerstats_topspeed _playerstats_averagespeed _playerstats_brakesused _playerstats_timeleftongate) (break `/Game/Blueprints/playerPerf` (`/Game/Blueprints/BPCar.playerStats` (stale `self.ReceiveActorBeginOverlap` _asbpcar))))
  (set `/Game/Blueprints/BPCar.playerStats` (make `/Game/Blueprints/playerPerf` _playerstats_collisions _playerstats_topspeed _playerstats_averagespeed _playerstats_brakesused (/ (+ _playerstats_timeleftongate (`self.gateTime`)) 2.0)) (stale `self.ReceiveActorBeginOverlap` _asbpcar)))

(event `self.ReceiveActorBeginOverlap`
  (params (OtherActor :type "Actor Object Reference"))
  ;[1 1 1] when car reaches gate, deactivate gate, play sound and call next gate activation
  (bind _asbpcar (cast `/Game/Blueprints/BPCar` OtherActor))
  (`self.setAverageTimeLeft`)
  (set `self.reached` true)
  (set `self.isActive` false)
  (`GameplayStatics.PlaySoundAtLocation` null (`self.K2_GetActorLocation`))
  (`self.activateNextGate`)
  (bind _outactors (`GameplayStatics.GetAllActorsWithInterface` "/Game/Blueprints/BI_GameEvents.BI_GameEvents_C"))
  (message `/Game/Blueprints/BI_GameEvents.[GLOBAL]GateReached` _outactors)
  (`self.K2_DestroyActor`))

(event `activateNextGate`
  ;[1 1 1] activate next gate and call it's countdown
  (bind _outactors (`GameplayStatics.GetAllActorsOfClass` "BPTimeGate_C")) ; only 2 gates at a time
  (bind _item (`KismetArrayLibrary.Array_Get` _outactors))
  (if (== _item self)
    (bind _item_2 (`KismetArrayLibrary.Array_Get` _outactors 1))
    (set `/Game/Blueprints/BPTimeGate.isActive` true _item_2)
    (`self.startCountdown` _item_2)
    (else
      (set `/Game/Blueprints/BPTimeGate.isActive` true _item)
      (`self.startCountdown` _item))))

(event `startCountdown`
  ;[1 1 1] if gate is activate, start timer countdown
  (`KismetSystemLibrary.K2_SetTimerDelegate` (delegate `timerReached`) (`self.gateTime`)))

(event `timerReached`
  ;[1 1 1] if gate is activate, start timer countdown
  ;;[1 0.004962 0.1006] GAME OVERRRR - this needs writing (game over event broadcast etc.?)
  (`self.[GLOBAL]RoundEnd`)
  (`KismetSystemLibrary.PrintString` "GAME OVER"))

(fn `UserConstructionScript`)