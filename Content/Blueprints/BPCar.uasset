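; BPCar is a car Blueprint driven by physics forces on its StaticMesh component from two input axes.
; The turning axis applies yaw torque as an acceleration change, so steering ignores mass.
; The movement axis applies a mass-dependent impulse along the actor's forward vector each time the axis event fires, with no delta-time scaling.
; BeginPlay, overlap and the construction script are empty.
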(event `InputAxis|turning`
  (params (AxisValue :type "Float (single-precision)"))
  (`PrimitiveComponent.AddTorque` (`self.StaticMesh`) (`KismetMathLibrary.MakeVector` 0.0 0.0 (* AxisValue 25.0)) "None" true))

(event `InputAxis|movement`
  (params (AxisValue :type "Float (single-precision)"))
  (`PrimitiveComponent.AddImpulse` (`self.StaticMesh`) (* (`KismetMathLibrary.GetForwardVector` (`self.K2_GetActorRotation`)) (* AxisValue 500000.0)) "None" false))

(event `self.ReceiveBeginPlay`)

(event `self.ReceiveActorBeginOverlap`
  (params (OtherActor :type "Actor Object Reference")))

(fn `UserConstructionScript`)