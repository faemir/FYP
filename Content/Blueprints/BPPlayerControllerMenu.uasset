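; Main menu player controller that blends the view to the Menucamera actor and shows the main menu widget.
; BeginPlay starts an eased camera blend, creates UIMainMenu after a short delay, then calls Possess following a Menupawn lookup.
; Tick polls the Exit button's hover state, playing or reversing a timeline that drives vignette intensity on the camera's post-process settings.
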(event `self.ReceiveBeginPlay`
  (bind _outactors (`GameplayStatics.GetAllActorsOfClass` "/Game/Blueprints/menucamera.menucamera_C"))
  (`self.SetViewTargetWithBlend` (`KismetArrayLibrary.Array_Get` _outactors) 1.0 "VTBlend_EaseInOut" 5.0)
  (`KismetSystemLibrary.Delay` 0.9)
  (bind _returnvalue (`|CreateWidget` "/Game/UI/UIMainMenu.UIMainMenu_C" self))
  (`UserWidget.AddToViewport` _returnvalue 0)
  (`GameplayStatics.GetAllActorsOfClass` "/Game/Blueprints/menupawn.menupawn_C")
  (`self.Possess` null))

(event `self.ReceiveTick`
  (params (DeltaSeconds :type "Float (single-precision)"))
  (bind _foundwidgets (`WidgetBlueprintLibrary.GetAllWidgetsOfClass` "/Game/UI/UIMainMenu.UIMainMenu_C" false))
  (bind _asuimain_menu (cast `/Game/UI/UIMainMenu` (`KismetArrayLibrary.Array_Get` _foundwidgets)))
  (bind _outactors (`GameplayStatics.GetAllActorsOfClass` "/Game/Blueprints/menucamera.menucamera_C"))
  (if (`Widget.IsHovered` (`/Game/UI/UIMainMenu.ExitButton` _asuimain_menu))
    (bind (_direction _vignette_value) (`Timeline|vignette exit` :!label _label)
      (:`Update`
        (setmembers `PostProcessSettings` :`StructRef` (`PostProcessComponent.Settings` (`/Game/Blueprints/menucamera.PostProcess` (`KismetArrayLibrary.Array_Get` _outactors))) :`VignetteIntensity` _vignette_value)))
    (else
      (goto _label :!via `Reverse`))))

(fn `UserConstructionScript`)