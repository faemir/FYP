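; Spline-based track actor that builds a randomly shaped piece of track in its Construction Script.
; It clears the spline, then fills it with stored locations and tangents from one of seven random presets: straight, curves or S-bends.
; It resizes TrackArray to match the point count, then AddNewChunk creates a spline mesh between each consecutive pair of points.
; Point positions are printed for debugging, and the event graph is empty.
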(event EventBeginPlay)

(event EventActorBeginOverlap
  (params (OtherActor :type Actor%20Object%20Reference)))

(event EventTick
  (params (DeltaSeconds :type Float%20%28single-precision%29)))

(fn ConstructionScript
  (bind _trackarray (Variables|Default|GettrackArray))
  ;[1 1 1] i think it has 2 spline points already by default it shouldnt keep
  (Spline|ClearSplinePoints (Variables|Default|GetSpline))
  (CallFunction|StoreSplinePoints)
  (Variables|Default|SetNumSplinePoints (Spline|GetNumberOfSplinePoints (Variables|Default|GetSpline)))
  (Math|Integer|CompareInt (Variables|Default|GetNumSplinePoints) (Utilities|Array|Length (Variables|Default|GettrackArray)) :!label _label
    (:>
      (Utilities|Array|Add (Variables|Default|GettrackArray) (Variables|Default|GettemplateStruct))
      (goto _label))
    (:==
      (for _index (range 0 (- (Variables|Default|GetNumSplinePoints) 2))
        (bind _output_get (Variables|Default|SetcurrentIndex _index))
        (CallFunction|AddNewChunk _output_get (Variables|Default|GettrackChunk))))
    (:<
      (Utilities|Array|RemoveIndex _trackarray (Utilities|Array|LastIndex _trackarray)))))

(fn AddNewChunk
  (params (currentIndex :type Integer) (trackMesh :type Static%20Mesh%20Object%20Reference))
  (LocalVariables|SettrackChunkStaticMesh trackMesh)
  (bind _output_get (LocalVariables|SetcurSplinePoint currentIndex))
  (LocalVariables|SetnextSplinePoint (Math|Integer|%(Integer) (+ _output_get 1) (Variables|Default|GetNumSplinePoints)))
  (LocalVariables|SetcurLoc (.Location (Spline|GetLocationandTangentatSplinePoint (Variables|Default|GetSpline) _output_get "Local")))
  (LocalVariables|SetcurTang (.Tangent (Spline|GetLocationandTangentatSplinePoint (Variables|Default|GetSpline) _output_get "Local")))
  (LocalVariables|SetnextLoc (.Location (Spline|GetLocationandTangentatSplinePoint (Variables|Default|GetSpline) (LocalVariables|GetnextSplinePoint) "Local")))
  (LocalVariables|SetnextTang (.Tangent (Spline|GetLocationandTangentatSplinePoint (Variables|Default|GetSpline) (LocalVariables|GetnextSplinePoint) "Local")))
  (bind _returnvalue (AddComponent|AddSplineMeshComponent false))
  (bind _output_get_2 (LocalVariables|SetchunkSplineMesh _returnvalue))
  (Components|StaticMesh|SetStaticMesh _output_get_2 (LocalVariables|GettrackChunkStaticMesh))
  (SplineMesh|SetStartandEnd (LocalVariables|GetchunkSplineMesh) (LocalVariables|GetcurLoc) (LocalVariables|GetcurTang) (LocalVariables|GetnextLoc) (LocalVariables|GetnextTang) :!class /Script/Engine.SplineMeshComponent)
  (SplineMesh|SetStartScale (LocalVariables|GetchunkSplineMesh) "(X=1.000,Y=1.000)" :!class /Script/Engine.SplineMeshComponent)
  (SplineMesh|SetEndScale (LocalVariables|GetchunkSplineMesh) "(X=1.000,Y=1.000)" :!class /Script/Engine.SplineMeshComponent))

(fn StoreSplinePoints
  (bind _trackpieceslist (Variables|Default|GettrackPiecesList))
  (bind _spline (Variables|Default|GetSpline))
  (Utilities|FlowControl|Sequence
    (:then_0
      (bind _output_get (LocalVariables|SettempChosenPieceArray (Utilities|Select :Index (Math|Random|RandomIntegerinRange 0 6) :Option%200 (.straight _trackpieceslist) :Option%201 (.rightcurvestrong _trackpieceslist) :Option%202 (.leftcurvestrong _trackpieceslist) :Option%203 (.rightcurvelight _trackpieceslist) :Option%204 (.leftcurvelight _trackpieceslist) :Option%205 (.sbendright _trackpieceslist) :Option%206 (.sbendleft _trackpieceslist))))
      (for (_array_element _array_index) _output_get
        (Spline|AddSplinePoint (Variables|Default|GetSpline) (.SplinePointLoc (Utilities|Struct|BreaksplinePoints _array_element)) "Local")
        (Spline|SetTangentatSplinePoint _spline _array_index (.SplinePointTan (Utilities|Struct|BreaksplinePoints _array_element)) "Local")
        (Development|PrintString (Utilities|String|ToString(Vector) (Spline|GetLocationatSplinePoint _spline _array_index "Local")))
        (Development|PrintString (Utilities|String|ToString(Transform) (Spline|GetTransformatSplinePoint _spline _array_index "Local" false)))))))