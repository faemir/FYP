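; Test actor that bends a single spline mesh along a spline component in the construction script.
; It sets the mesh start and end from the first and last spline points' local location and tangent, so intermediate points do not shape it.
; A disconnected branch that would append two offset spline points before the mesh update never runs, and the event graph is empty.
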(event `self.ReceiveBeginPlay`)

(event `self.ReceiveActorBeginOverlap`
  (params (OtherActor :type "Actor Object Reference")))

(event `self.ReceiveTick`
  (params (DeltaSeconds :type "Float (single-precision)")))

(fn `UserConstructionScript`
  (bind _spline (`self.Spline`))
  (bind (_location _tangent) (`SplineComponent.GetLocationAndTangentAtSplinePoint` _spline 0 "Local"))
  (bind (_location_2 _tangent_2) (`SplineComponent.GetLocationAndTangentAtSplinePoint` _spline (- (`SplineComponent.GetNumberOfSplinePoints` _spline) 1) "Local"))
  (`SplineMeshComponent.SetStartAndEnd` (`self.SplineMesh`) _location _tangent _location_2 _tangent_2))