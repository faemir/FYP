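; BPChunkManager builds the level as a chain of spawned BPChunk actors tracked in the LevelChunks array.
; It creates three chunks at one-second intervals on BeginPlay, the first at world origin.
; Each later chunk spawns at the last spline point of the previous chunk's final segment and attaches to the manager's root.
; GateReached removes index 1 from the array, without destroying that actor, then appends a new chunk.
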(event `self.ReceiveBeginPlay`
  (`self.addChunk`)
  (`KismetSystemLibrary.Delay` 1.0)
  ;[1 1 1] need second but also need to add handling it properly
  (`self.addChunk`)
  (`KismetSystemLibrary.Delay` 1.0)
  (`self.addChunk`))

(event `self.ReceiveActorBeginOverlap`
  (params (OtherActor :type "Actor Object Reference")))

(event `self.ReceiveTick`
  (params (DeltaSeconds :type "Float (single-precision)")))

(event `/Game/Blueprints/BI_GameEvents.[GLOBAL]GateReached`
  (bind _levelchunks (`self.levelChunks`))
  ;[1 1 1] when gate is reached, set chunk 1 to chunk 0 and then clear it from chunk 1
  (`KismetArrayLibrary.Array_Set` _levelchunks 0 (`KismetArrayLibrary.Array_Get` _levelchunks))
  (`self.removeChunk` 1)
  (`self.addChunk`))

(fn `addChunk`
  (bind _levelchunks (`self.levelChunks`))
  (bind _segments (`/Game/Blueprints/BPChunk.Segments` (`KismetArrayLibrary.Array_Get` _levelchunks (- (`KismetArrayLibrary.Array_Length` _levelchunks) 1))))
  (bind _spline (`/Game/Blueprints/BPSpline.Spline` (`KismetArrayLibrary.Array_Get` _segments (- (`KismetArrayLibrary.Array_Length` _segments) 1))))
  (bind _returnvalue (`SplineComponent.GetTransformAtSplinePoint` _spline (- (`SplineComponent.GetNumberOfSplinePoints` _spline) 1) "World" false))
  ;[1 1 1] need to add tracking which chunk is which
  (if (== 0 (`KismetArrayLibrary.Array_Length` (`self.levelChunks`)))
    (bind _returnvalue_2 (`|SpawnActorFromClass` "/Game/Blueprints/BPChunk.BPChunk_C" (`KismetMathLibrary.MakeTransform` (0.0 0.0 0.0)) "Undefined" "OverrideRootScale"))
    (`self.K2_AttachRootComponentTo` _returnvalue_2 (`self.DefaultSceneRoot`) "None" "KeepWorldPosition" true)
    (`KismetArrayLibrary.Array_Add` (`self.levelChunks`) _returnvalue_2)
    (else
      (`KismetSystemLibrary.PrintString` (`KismetStringLibrary.Conv_TransformToString` _returnvalue))
      (bind _returnvalue_3 (`|SpawnActorFromClass` "/Game/Blueprints/BPChunk.BPChunk_C" _returnvalue "Undefined" "OverrideRootScale"))
      (`self.K2_AttachRootComponentTo` _returnvalue_3 (`self.DefaultSceneRoot`) "None" "KeepWorldPosition" true)
      (`KismetArrayLibrary.Array_Add` (`self.levelChunks`) _returnvalue_3))))

(fn `removeChunk`
  (params (chunkToRemove :type Integer))
  (`KismetArrayLibrary.Array_Remove` (`self.levelChunks`) chunkToRemove))

(fn `UserConstructionScript`)