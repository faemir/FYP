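; Live Editor script that tunes a BPCar's physics from MIDI-style note and control-change bindings.
; OnInit registers the bindings, and OnAssign targets the car selected in the editor.
; Adjustment events add scaled deltas to turning, friction, acceleration and mesh linear/angular damping, clamping friction and damping and mirroring values locally.
; CacheState and LoadFromState handle only a Light variable that this file never assigns a light to, so neither saves car values.
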(event `/Game/Blueprints/BP_LiveEditor_Lighting.OnShutdown`
  (set `self.Light` null))

(event `OnAssign`
  (params (Delta :type Integer))
  ;[1 1 1] Assign Car to Script
  (bind _returnvalue (`LiveEditorKismetLibrary.GetSelectedEditorObject`))
  (bind _asbpcar (cast `/Game/Blueprints/BPCar` _returnvalue))
  (set `self.BPCar` _asbpcar)
  (`self.CacheState`))

(event `/Game/Blueprints/BP_LiveEditor_Lighting.OnInit`
  ;[1 1 1] register key assigns
  (`LiveEditorKismetLibrary.RegisterForLiveEditEvent` "OnAssign" "Assign Car" (`|MakeArray` "NoteOnOff" :!type "ELiveEditControllerType Enum"))
  (`LiveEditorKismetLibrary.RegisterForLiveEditEvent` "OnAdjustTurning" "Turning" (`|MakeArray` "ControlChangeFixed" "ControlChangeFixed" :!type "ELiveEditControllerType Enum"))
  (`LiveEditorKismetLibrary.RegisterForLiveEditEvent` "OnAdjustTurnFriction" "Friction" (`|MakeArray` "ControlChangeFixed" "ControlChangeFixed" :!type "ELiveEditControllerType Enum"))
  (`LiveEditorKismetLibrary.RegisterForLiveEditEvent` "OnAdjustAccel" "Acceleration" (`|MakeArray` "ControlChangeFixed" "ControlChangeFixed" :!type "ELiveEditControllerType Enum"))
  (`LiveEditorKismetLibrary.RegisterForLiveEditEvent` "OnAdjustLinearDamp" "Linear Dampening" (`|MakeArray` "ControlChangeFixed" "ControlChangeFixed" :!type "ELiveEditControllerType Enum"))
  (`LiveEditorKismetLibrary.RegisterForLiveEditEvent` "OnAdjustAngularDamp" "Angular Dampening" (`|MakeArray` "ControlChangeFixed" "ControlChangeFixed" :!type "ELiveEditControllerType Enum")))

(event `OnAdjustTurning`
  (params (Delta :type Integer))
  (bind _bpcar (`self.BPCar`))
  ;[1 1 1] Physics Values
  (if (!= _bpcar null)
    (bind _output_get (set `/Game/Blueprints/BPCar.turning` (+ (* (`KismetMathLibrary.Conv_IntToDouble` Delta) 50.0) (`/Game/Blueprints/BPCar.turning` _bpcar)) _bpcar))
    (set `self.Turning` _output_get)))

(event `OnAdjustTurnFriction`
  (params (Delta :type Integer))
  (bind _bpcar (`self.BPCar`))
  ;[1 1 1] Physics Values
  (if (!= _bpcar null)
    (bind _output_get (set `/Game/Blueprints/BPCar.turnFriction` (`KismetMathLibrary.FClamp` (+ (* (`KismetMathLibrary.Conv_IntToDouble` Delta) 0.05) (`/Game/Blueprints/BPCar.turnFriction` _bpcar)) 0.0 50.0) _bpcar))
    (set `self.TurnFriction` _output_get)))

(event `OnAdjustAccel`
  (params (Delta :type Integer))
  (bind _bpcar (`self.BPCar`))
  ;[1 1 1] Physics Values
  (if (!= _bpcar null)
    (bind _output_get (set `/Game/Blueprints/BPCar.AccelVal` (+ (* (`KismetMathLibrary.Conv_IntToDouble` Delta) 5000.0) (`/Game/Blueprints/BPCar.AccelVal` _bpcar)) _bpcar))
    (set `self.AccelVal` _output_get)))

(event `OnAdjustLinearDamp`
  (params (Delta :type Integer))
  (bind _bpcar (`self.BPCar`))
  (bind _returnvalue (`PrimitiveComponent.GetLinearDamping` (`/Game/Blueprints/BPCar.StaticMesh` _bpcar)))
  ;[1 1 1] Physics Values
  (if (!= _bpcar null)
    (`PrimitiveComponent.SetLinearDamping` (`/Game/Blueprints/BPCar.StaticMesh` _bpcar) (`KismetMathLibrary.FClamp` (+ (* (`KismetMathLibrary.Conv_IntToDouble` Delta) 0.05) _returnvalue) 0.0 999.0))
    (set `self.LinearDamp` _returnvalue)))

(event `OnAdjustAngularDamp`
  (params (Delta :type Integer))
  (bind _bpcar (`self.BPCar`))
  (bind _returnvalue (`PrimitiveComponent.GetAngularDamping` (`/Game/Blueprints/BPCar.StaticMesh` _bpcar)))
  ;[1 1 1] Physics Values
  (if (!= _bpcar null)
    (`PrimitiveComponent.SetAngularDamping` (`/Game/Blueprints/BPCar.StaticMesh` _bpcar) (`KismetMathLibrary.FClamp` (+ (* (`KismetMathLibrary.Conv_IntToDouble` Delta) 0.1) _returnvalue) 0.0 999.0))
    (set `self.AngularDamp` _returnvalue)))

(fn `CacheState`
  (bind _light (`self.Light`))
  (bind _lightcomponent (`Light.LightComponent` _light))
  (bind (_h _s _v) (`KismetMathLibrary.RGBToHSV` (`KismetMathLibrary.Conv_ColorToLinearColor` (`LightComponentBase.LightColor` _lightcomponent))))
  (`/Engine/EditorBlueprintResources/StandardMacros.IsValid` _light
    (:`Is Valid`
      (set `self.H` _h)
      (set `self.S` _s)
      (set `self.V` _v)
      (set `self.Brightness` (`LightComponentBase.Intensity` _lightcomponent))
      (bind _asspot_light (cast `SpotLight` _light))
      (bind _spotlightcomponent (`SpotLight.SpotLightComponent` _asspot_light))
      (set `self.InnerConeAngle` (`SpotLightComponent.InnerConeAngle` _spotlightcomponent))
      (set `self.OuterConeAngle` (`SpotLightComponent.OuterConeAngle` _spotlightcomponent)))))

(fn `LoadFromState`
  (bind _light (`self.Light`))
  (`/Engine/EditorBlueprintResources/StandardMacros.IsValid` _light
    (:`Is Valid`
      (`LightComponent.SetLightColor` _light (`KismetMathLibrary.HSVToRGB` (`self.H`) (`self.S`) (`self.V`)) true)
      (bind _asspot_light (cast `SpotLight` (`self.Light`)))
      (`SpotLightComponent.SetInnerConeAngle` _asspot_light (`self.InnerConeAngle`))
      (`SpotLightComponent.SetOuterConeAngle` _asspot_light (`self.OuterConeAngle`)))))