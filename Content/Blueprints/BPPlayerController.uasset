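; Player controller for a driving game that creates the vehicle HUD, blends the view to the car and handles game over.
; Tick polls GameOver to show a UI-only game-over screen once, and the chunk manager's ChangeColour flag for gate passes.
; A gate pass picks a random colour and calls MoveBackP on the manager.
; A timeline sweeps the colour across track spline meshes through a dynamic material's pixel-depth lerp.
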(event `self.ReceiveBeginPlay`
  (bind _returnvalue (`GameplayStatics.GetPlayerController` 0))
  ;[1 1 1] Create player UI and pan smoothly to the car camera
  (bind _returnvalue_2 (`|CreateWidget` "/Game/UI/vehicleUI.vehicleUI_C"))
  (`UserWidget.AddToViewport` _returnvalue_2 0)
  (bind _outactors (`GameplayStatics.GetAllActorsOfClass` "/Game/Blueprints/BPCar.BPCar_C"))
  (`self.SetViewTargetWithBlend` (`KismetArrayLibrary.Array_Get` _outactors) 1.0)
  (`|ExecutionSequence`
    (:`then_0`
      (goto _label_3 :!via `Reset`))
    (:`then_1`
      (bind _outactors_2 (`GameplayStatics.GetAllActorsOfClass` "/Game/Blueprints/BPChunkManager.BPChunkManager_C" :!label _label))
      (`/Game/Blueprints/BPChunkManager.moveBackP` (`KismetArrayLibrary.Array_Get` _outactors_2)))))

(event `self.ReceiveTick`
  (params (DeltaSeconds :type "Float (single-precision)"))
  (bind _returnvalue (`GameplayStatics.GetPlayerController` 0))
  ;[1 1 1] Colour change on gate pass
  (`|ExecutionSequence`
    (:`then_0`
      (bind _outactors (`GameplayStatics.GetAllActorsOfClass` "/Game/Blueprints/BPChunkManager.BPChunkManager_C"))
      (if (`FYPChunkManager.changeColour` (`KismetArrayLibrary.Array_Get` _outactors))
        (`/Engine/EditorBlueprintResources/StandardMacros.DoOnce` false :!label _label_2
          (:`Completed`
            (`|ExecutionSequence`
              (:`then_0`
                (`self.changecol`))
              (:`then_1`
                (goto _label)))))))
    (:`then_1`
      ;[1 1 1] GameOver UI
      (if (`self.gameOver`)
        (`/Engine/EditorBlueprintResources/StandardMacros.DoOnce` false :!label _label_3
          (:`Completed`
            (`WidgetLayoutLibrary.RemoveAllWidgets`)
            (bind _returnvalue_2 (`|CreateWidget` "/Game/UI/UIGameOver.UIGameOver_C"))
            (`UserWidget.AddToViewport` _returnvalue_2 0)
            ;;[1 1 1] this is to fix mouse input
            (`self.DisableInput` (`self.K2_GetPawn` _returnvalue) _returnvalue)
            (set `self.bShowMouseCursor` true)
            (`WidgetBlueprintLibrary.SetInputMode_UIOnlyEx` _returnvalue _returnvalue_2 true)))))))

(event `changecol`
  (bind _dynamicmaterial (`self.DynamicMaterial`))
  ;[1 1 1] Colour change on gate pass
  (set `FYPChunkManager.changeColour` false (`KismetArrayLibrary.Array_Get` (stale `self.ReceiveTick` _outactors)))
  (bind _output_get (set `self.newCol` (make `LinearColor` (`KismetMathLibrary.RandomFloatInRange` 0.0 1.0) (`KismetMathLibrary.RandomFloatInRange` 0.0 1.0) (`KismetMathLibrary.RandomFloatInRange` 0.0 1.0) 1.0)))
  (`KismetSystemLibrary.PrintString` (`KismetStringLibrary.Conv_ColorToString` _output_get) true true (struct :`G` 0.66 :`B` 1.0 :`A` 1.0) 4.0)
  (bind _outactors (`GameplayStatics.GetAllActorsOfClass` "/Script/FYP.FYPChunk"))
  (for _array_element _outactors
    (for _array_element_2 (`FYPChunk.Segments` _array_element)
      (for _array_element_3 (`self.K2_GetComponentsByClass` _array_element_2 "/Script/Engine.SplineMeshComponent")
        (bind _returnvalue (`PrimitiveComponent.CreateDynamicMaterialInstance` _array_element_3 0 null))
        (bind _output_get_2 (set `self.DynamicMaterial` _returnvalue))
        (`MaterialInstanceDynamic.SetVectorParameterValue` _output_get_2 "Lerp Colour1" (`self.newCol`))
        (`TimelineComponent.SetPlayRate` (`self.Timeline_0`) 0.25)
        (bind (_direction _newtrack_0) (`Timeline|Timeline_0` :!via `PlayFromStart`)
          (:`Update`
            (`MaterialInstanceDynamic.SetScalarParameterValue` (`self.DynamicMaterial`) "PixelDepth Factor" (`KismetMathLibrary.Lerp` 0.0 5000000.0 _newtrack_0))
            (bind _outactors_2 (`GameplayStatics.GetAllActorsOfClass` "/Script/FYP.FYPChunk"))
            (for _array_element_4 _outactors_2
              (for _array_element_5 (`FYPChunk.Segments` _array_element_4)
                (for _array_element_6 (`self.K2_GetComponentsByClass` _array_element_5 "/Script/Engine.SplineMeshComponent")
                  (`PrimitiveComponent.SetMaterial` _array_element_6 0 (`self.DynamicMaterial`))
                  (goto _label_2 :!via `Reset`)))))
          (:`Finished`
            (`MaterialInstanceDynamic.SetVectorParameterValue` _dynamicmaterial "Lerp Colour2" (`self.newCol`))
            (`MaterialInstanceDynamic.SetScalarParameterValue` _dynamicmaterial "PixelDepth Factor" 0.0)))))))

(fn `UserConstructionScript`)